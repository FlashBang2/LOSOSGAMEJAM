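; Player controller that handles Enhanced Input for movement, interaction and the escape menu.
; It registers the controls mapping context, then moves the pawn along yaw-based control-rotation axes.
; Escape toggles the menu widget after a short delay, and interact messages overlapping A_escape and A_item actors, triggering the opening-sequence call for escapes.
; InCutscene blocks all three actions, while InEscapeMenu blocks movement and interaction.
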(event `self.ReceiveBeginPlay`
  (bind _returnvalue (pcsubsystem `EnhancedInputLocalPlayerSubsystem` self))
  (`/Engine/EditorBlueprintResources/StandardMacros.IsValid` _returnvalue
    (:`Is Valid`
      (`EnhancedInputSubsystemInterface.AddMappingContext` _returnvalue "/Game/InputsMapping/IMC_controls.IMC_controls" 0 (struct)))))

(event `EnhancedInput|/Game/InputsMapping/IA_move`
  (params (ActionValue :type "Vector2D Structure") (ElapsedSeconds :type "Float (double-precision)") (TriggeredSeconds :type "Float (double-precision)") (InputAction :type "InputAction Object Reference" :default "/Game/InputsMapping/IA_move.IA_move"))
  (bind _returnvalue (`self.K2_GetPawn`))
  (bind _returnvalue_2 (`self.K2_GetPawn`))
  (bind (_returnvalue_roll _returnvalue_pitch _returnvalue_yaw) (`KismetMathLibrary.BreakRotator` (`Pawn.GetControlRotation` _returnvalue)))
  (bind (_returnvalue_roll_2 _returnvalue_pitch_2 _returnvalue_yaw_2) (`KismetMathLibrary.BreakRotator` (`Pawn.GetControlRotation` _returnvalue)))
  (:`Triggered`
    (if (and (not (`self.InCutscene`)) (not (`self.InEscapeMenu`)))
      (`|ExecutionSequence`
        (:`then_0`
          (`Pawn.AddMovementInput` _returnvalue_2 (`KismetMathLibrary.GetRightVector` (`KismetMathLibrary.MakeRotator` _returnvalue_roll 0.0 _returnvalue_yaw)) ActionValue_X false))
        (:`then_1`
          (`Pawn.AddMovementInput` _returnvalue_2 (`KismetMathLibrary.GetForwardVector` (`KismetMathLibrary.MakeRotator` 0.0 0.0 _returnvalue_yaw_2)) ActionValue_Y false))))))

(event `EnhancedInput|/Game/InputsMapping/IA_interact`
  (params (ActionValue :type Boolean) (ElapsedSeconds :type "Float (double-precision)") (TriggeredSeconds :type "Float (double-precision)") (InputAction :type "InputAction Object Reference" :default "/Game/InputsMapping/IA_interact.IA_interact"))
  (bind _returnvalue (`self.K2_GetPawn`))
  (bind _output (`|GetArrayItem` (`self.GetOverlappingActors` _returnvalue "/Game/Actors/A_item.A_item_C")))
  (bind _output_2 (`|GetArrayItem` (`self.GetOverlappingActors` _returnvalue "/Game/Actors/A_escape.A_escape_C")))
  (:`Triggered`
    (if (and (not (`self.InCutscene`)) (not (`self.InEscapeMenu`)))
      (`|ExecutionSequence`
        (:`then_0`
          (`/Engine/EditorBlueprintResources/StandardMacros.IsValid` _output_2
            (:`Is Valid`
              (bind _escape (message `/Game/Interfaces/I_escape.GetEscape` _output_2))
              (`/Game/Actors/A_escape.OpeningSequenceStarted` _escape))))
        (:`then_1`
          (`/Engine/EditorBlueprintResources/StandardMacros.IsValid` _output
            (:`Is Valid`
              (message `/Game/Interfaces/I_item.GetItem` _output))))))))

(event `EnhancedInput|/Game/InputsMapping/IA_escape`
  (params (ActionValue :type Boolean) (ElapsedSeconds :type "Float (double-precision)") (TriggeredSeconds :type "Float (double-precision)") (InputAction :type "InputAction Object Reference" :default "/Game/InputsMapping/IA_escape.IA_escape"))
  (bind _escapemenu (`self.EscapeMenu`))
  (:`Triggered`
    (if (not (`self.InCutscene`))
      (if (`self.InEscapeMenu`)
        (`KismetSystemLibrary.Delay` 0.2)
        (set `self.InEscapeMenu` false)
        (`/Engine/EditorBlueprintResources/StandardMacros.IsValid` _escapemenu
          (:`Is Valid`
            (`Widget.RemoveFromParent` _escapemenu)))
        (else
          (`KismetSystemLibrary.Delay` 0.2)
          (bind _returnvalue (`|CreateWidget` "/Game/Widgets/W_escapeMenu.W_escapeMenu_C"))
          (set `self.EscapeMenu` _returnvalue)
          (set `self.InEscapeMenu` true)
          (`UserWidget.AddToViewport` (`self.EscapeMenu`) 1))))))

(fn `GetPlayerController`
  (returns (PlayerController :type "/Game/PlayerControllers/PC_controller Object Reference"))
  (return self))

(fn `UserConstructionScript`)